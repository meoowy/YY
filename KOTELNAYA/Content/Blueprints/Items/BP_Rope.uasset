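; BP_Rope is an interactable rope that the player cuts with a Knife to regain movement.
; On BeginPlay it creates a hidden interaction prompt widget, shown and collapsed as focus is gained and lost.
; Interact checks the first-person character's inventory for the Knife, consumes it, sets CanMove, updates the HUD hint about clearing the path, then destroys the rope and plays a 2D sound.
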(event EventOnFocusReceived
  (Widget|SetVisibility (Variables|Default|GetWidget) "Visible"))

(event EventOnFocusLost
  (Widget|SetVisibility (Variables|Default|GetWidget) "Collapsed"))

(event EventBeginPlay
  (bind _returnvalue (UserInterface|CreateWidget "/Game/Blueprints/UI/W_InteractionPrompt.W_InteractionPrompt_C" 0 (Variables|Default|GetMassage)))
  (bind _output_get (Variables|Default|SetWidget _returnvalue))
  (UserInterface|Viewport|AddtoViewport _output_get 0)
  (Widget|SetVisibility _output_get "Collapsed"))

(fn ConstructionScript)

(fn GetInteractionActionText
  (return ""))

(fn Interact
  (params (InstigatorPawn :type Pawn%20Object%20Reference))
  (bind _asbp_first_person_character (Utilities|Casting|CastToBP_FirstPersonCharacter InstigatorPawn))
  (if (Class|IHInventoryComponent|HasItem (Variables|/Game/FirstPerson/Blueprints/BP_FirstPersonCharacter.BP_FirstPersonCharacter_C|GetIHInventory _asbp_first_person_character) "Knife" 1)
    (Default|UpdateHint (Variables|/Game/FirstPerson/Blueprints/BP_FirstPersonCharacter.BP_FirstPersonCharacter_C|GetHud _asbp_first_person_character) "Надо найти чем расчистить путь")
    (Class|IHInventoryComponent|RemoveItem (Variables|/Game/FirstPerson/Blueprints/BP_FirstPersonCharacter.BP_FirstPersonCharacter_C|GetIHInventory _asbp_first_person_character) "Knife" 1)
    (Variables|/Game/FirstPerson/Blueprints/BP_FirstPersonCharacter.BP_FirstPersonCharacter_C|SetCanMove _asbp_first_person_character true)
    (Actor|DestroyActor)
    (Audio|PlaySound2D (Variables|Default|GetSound) 1.0 1.0 0.0 0 0)
    (return false)))