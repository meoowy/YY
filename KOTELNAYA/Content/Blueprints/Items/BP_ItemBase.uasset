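; BP_ItemBase is a base pickup item that the player can focus and interact with to add it to their inventory.
; On BeginPlay it creates a hidden W_InteractionPrompt widget, which focus events show and collapse.
; Interact looks up the item's DT_GameItems row, passes its ID to the instigator's IHInventoryComponent, and destroys the actor when TryAddItem returns zero.
; The action-text getter still contains a debug print.
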(event EventOnFocusReceived
  (Widget|SetVisibility (Variables|Default|GetWidget) "Visible"))

(event EventOnFocusLost
  (Widget|SetVisibility (Variables|Default|GetWidget) "Collapsed"))

(event EventBeginPlay
  (bind _returnvalue (UserInterface|CreateWidget "/Game/Blueprints/UI/W_InteractionPrompt.W_InteractionPrompt_C" 0 (Variables|Default|GetMassage)))
  (bind _output_get (Variables|Default|SetWidget _returnvalue))
  (UserInterface|Viewport|AddtoViewport _output_get 0)
  (Widget|SetVisibility _output_get "Collapsed"))

(fn ConstructionScript)

(fn NewFunction
  (params (self2 :type User%20Widget%20Object%20Reference))
  (UserInterface|Viewport|AddtoViewport self2 0))

(fn GetInteractionActionText
  (Development|PrintText "Hello")
  (return (Utilities|Text|FormatText "{var1}{var2}" (Variables|/Script/InteractionSystem.IHInteractableTargetComponent|GetDefaultInteractionText (Variables|Default|GetIHInteractableTarget)))))

(fn Interact
  (params (InstigatorPawn :type Pawn%20Object%20Reference))
  (bind _returnvalue (Utilities|GetDataTableRow "/Game/Blueprints/Inventory/DT_GameItems.DT_GameItems" (Variables|Default|GetName))
    (:then
      (bind _returnvalue_2 (Class|IHInventoryComponent|TryAddItem (Actor|GetComponentbyClass InstigatorPawn "/Script/InventorySystem.IHInventoryComponent") (.ItemID (Utilities|Struct|BreakIHItemDefinition _returnvalue)) 1))
      (if (== _returnvalue_2 0)
        (Actor|DestroyActor))
      (return false))))