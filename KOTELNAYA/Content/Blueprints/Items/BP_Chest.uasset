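; BP_Chest is an interactable chest that presents a code-entry panel to the player.
; On BeginPlay it creates a hidden W_CodePanel, passing the correct answer and itself, plus a hidden W_InteractionPrompt.
; Focus events toggle the prompt, and Interact hides it, shows the panel and calls StartEntering.
; Answer checking and any opening behavior are not in this Blueprint's graphs.
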(event EventOnFocusReceived
  (Widget|SetVisibility (Variables|Default|GetWidgetPromt) "Visible"))

(event EventOnFocusLost
  (Widget|SetVisibility (Variables|Default|GetWidgetPromt) "Collapsed"))

(event EventBeginPlay
  (bind _returnvalue (UserInterface|CreateWidget "/Game/Blueprints/UI/W_CodePanel.W_CodePanel_C" 0 (Variables|Default|GetAnswer) self))
  (bind _output_get (Variables|Default|SetWidget _returnvalue))
  (UserInterface|Viewport|AddtoViewport _output_get 0)
  (Widget|SetVisibility _output_get "Collapsed")
  (bind _returnvalue_2 (UserInterface|CreateWidget "/Game/Blueprints/UI/W_InteractionPrompt.W_InteractionPrompt_C" 0 (Variables|Default|GetMassage)))
  (bind _output_get_2 (Variables|Default|SetWidgetPromt _returnvalue_2))
  (UserInterface|Viewport|AddtoViewport _output_get_2 0)
  (Widget|SetVisibility _output_get_2 "Collapsed"))

(fn ConstructionScript)

(fn GetInteractionActionText
  (return ""))

(fn Interact
  (params (InstigatorPawn :type Pawn%20Object%20Reference))
  (bind _widget (Variables|Default|GetWidget))
  (Widget|SetVisibility (Variables|Default|GetWidgetPromt) "Collapsed")
  (Widget|SetVisibility _widget "Visible")
  (Default|StartEntering _widget)
  (return false))